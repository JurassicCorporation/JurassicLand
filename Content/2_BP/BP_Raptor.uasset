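; Playable raptor character for dinosaur combat, with tail, bite and roar attacks, a cooldown flamethrower and timed stat buffs.
; Inputs call server events that multicast montages, state flags and effects; flame breath repeatedly spawns projectiles while active.
; A timeline-driven sphere trace acquires a lock-on target, which Tick turns the controller toward.
; Hit multicast handles stagger and slow-motion death, but damage-type logic is disconnected, so AnyDamage only prints.
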(event `self.ReceiveAnyDamage`
  (params (Damage :type "Float (single-precision)") (DamageType :type "DamageType Object Reference") (InstigatedBy :type "Controller Object Reference") (DamageCauser :type "Actor Object Reference"))
  ;[1 1 1] Apply Damage & Die
  (`KismetSystemLibrary.PrintString` "DAm it!"))

(event `fireEffectServer`
  (`self.fireEffectMulticast`))

(event `fireEffectMulticast`
  (`GameplayStatics.SpawnEmitterAttached` null (`self.CapsuleComponent`) "None" (0.0 110.0 0.0)))

(event `iceHitEffectMultiCast`
  (`GameplayStatics.SpawnEmitterAtLocation` null (`self.K2_GetActorLocation`) (struct) (0.5 0.5 0.5)))

(event `self.ReceiveBeginPlay`
  ;[0.07669 0.9741 1] BeginPlay (Initial Setting)
  (bind _asbp_lsh_bphpwidget (cast `/Game/2_BP/Widget/BP_LSH_BPHPWidget` (`WidgetComponent.GetWidget` (`self.HP_Bar`))))
  (set `/Game/2_BP/Widget/BP_LSH_BPHPWidget.Dino_ref` self _asbp_lsh_bphpwidget)
  (set `CharacterMovementComponent.MaxWalkSpeed` (* 150.0 (`self.SpeedStat`)) (`self.CharacterMovement`))
  (set `self.HP` (`KismetMathLibrary.FTrunc` (* 30.0 (`self.DefenceStat`))))
  (`self.SpecialSkillEffectMaker`)
  (`self.buffSkillEffectMaker`)
  (`Timeline|Timeline_0` :!via `PlayFromStart`
    (:`Update`
      (`self.LockOnTarget`
        (:`then`)
        (:`else`
          (bind (_outhit _returnvalue) (`KismetSystemLibrary.SphereTraceSingleForObjects` (`self.K2_GetActorLocation`) (0.0 0.0 0.0) 2000.0 (`|MakeArray` "ObjectTypeQuery3" :!type "EObjectTypeQuery Enum")))
          (if _returnvalue
            (set `self.LockOnTarget` (`.HitActor` (`GameplayStatics.BreakHitResult` _outhit)))))))))

(event `hitEffectServer`
  (`self.hitEffectMulticast`))

(event `hitEffectMulticast`
  (if (<= (`self.State_HP`) 0.0)
    ;[0 0.06098 1] Die
    (`GameplayStatics.PlayWorldCameraShake` "/Game/2_BP/CameraShaking/BP_GetHit.BP_GetHit_C" (`self.K2_GetActorLocation`) 0.0 2000.0)
    (`SkeletalMeshComponent.PlayAnimation` (`self.Mesh`) "/Game/7_MISC/Animation/BlueTRex/BS/BlueTRex_A_012_TRexSue_Die_Anim.BlueTRex_A_012_TRexSue_Die_Anim" false)
    (`GameplayStatics.SetGlobalTimeDilation` 0.5)
    (else
      ;[1 0.304 0.6201] Damage
      (set `CharacterMovementComponent.MaxWalkSpeed` 0.0 (`self.CharacterMovement`))
      (set `self.bUseControllerRotationYaw` false)
      (`KismetSystemLibrary.Delay` 1.0)
      (set `self.bIsNoHit` true))))

(event `InputAxisKey|MouseX`
  (params (AxisValue :type "Float (single-precision)"))
  ;[0.1665 0.08562 0.2292] In Place Turn
  (if (== (`KismetMathLibrary.VSize` (`MovementComponent.Velocity` (`self.CharacterMovement`))) 0.0) :!label _label
    (`|ExecutionSequence`
      (:`then_0`
        (if (>= AxisValue 0.7)
          (set `self.bTurnRight` true)
          (set `self.bTurnLeft` false)
          (else
            (set `self.bTurnRight` false))))
      (:`then_1`
        (if (<= AxisValue -0.7)
          (set `self.bTurnLeft` true)
          (set `self.bTurnRight` false)
          (else
            (set `self.bTurnLeft` false)))))
    (else
      (set `self.bTurnLeft` false)
      (set `self.bTurnRight` false))))

(event `EnhancedInput|/Game/7_MISC/Input/IA_PlayerLook`
  (params (ActionValue :type "Vector2D Structure") (ElapsedSeconds :type "Float (double-precision)") (TriggeredSeconds :type "Float (double-precision)") (InputAction :type "InputAction Object Reference" :default "/Game/7_MISC/Input/IA_PlayerLook.IA_PlayerLook"))
  ;[0.1665 0.08562 0.2292] In Place Turn
  (:`Triggered`
    (goto _label)))

(event `self.ReceiveTick`
  (params (DeltaSeconds :type "Float (single-precision)"))
  (bind _returnvalue (`self.GetController`))
  ;[0.15 0.227 0.3419] LockOnSystem
  (`self.LockOnTarget`
    (:`then`
      (`/Engine/EditorBlueprintResources/StandardMacros.IsValid` _returnvalue
        (:`Is Valid`
          (`Controller.SetControlRotation` _returnvalue (`KismetMathLibrary.FindLookAtRotation` (`SceneComponent.GetSocketLocation` (`self.PlayerBody`) "bn_Neck1_8") (`self.K2_GetActorLocation` (`self.LockOnTarget`)))))))
    (:`else`)))

(event `EnhancedInput|/Game/7_MISC/Input/IA_Basic_TailAttack`
  (params (ActionValue :type Boolean) (ElapsedSeconds :type "Float (double-precision)") (TriggeredSeconds :type "Float (double-precision)") (InputAction :type "InputAction Object Reference" :default "/Game/7_MISC/Input/IA_Basic_TailAttack.IA_Basic_TailAttack"))
  ;[1 1 1] TailAttack
  (:`Started`
    (`self.TailAttack_Server` :!label _label_2)))

(event `Key|One`
  (params (Key :type "Key Structure"))
  ;[1 1 1] TailAttack
  (:`Pressed`
    (goto _label_2)))

(event `flameProjectileSpawner`
  (bind (_returnvalue_location _returnvalue_rotation) (`KismetMathLibrary.BreakTransform` (`SceneComponent.K2_GetComponentToWorld` (`self.SkillNiaEffect`))))
  ;[1 0.5647 0.3005] 화염방사 충돌체 생성
  (if (`self.bFlameOnOff`) :!label _label_3
    (`|SpawnActorFromClass` "/Game/2_BP/BP_FlameProjectile.BP_FlameProjectile_C" (`KismetMathLibrary.MakeTransform` _returnvalue_location _returnvalue_rotation (10.0 10.0 10.0)) "AlwaysSpawn" "MultiplyWithRoot" self null)
    (`KismetSystemLibrary.Delay` 0.2)
    (goto _label_3)))

(event `TailAttack_Server`
  ;[1 1 1] TailAttack
  (`self.TailAttack_Multicast`))

(event `TailAttack_Multicast`
  ;[1 1 1] TailAttack
  (if (not (`self.bTailAttack`))
    (set `self.bTailAttack` true)
    (set `CharacterMovementComponent.MaxWalkSpeed` 0.0 (`self.CharacterMovement`))
    (set `self.bUseControllerRotationYaw` false)))

(event `TailAttackEnd`
  ;[1 1 1] TailAttack
  (if (`self.bTailAttack`)
    (set `self.bTailAttack` false)
    (set `CharacterMovementComponent.MaxWalkSpeed` (* 150.0 (`self.speedStat`)) (`self.CharacterMovement`))
    (`SkeletalMeshComponent.SetAnimationMode` (`self.Mesh`) "AnimationBlueprint")
    (set `self.bUseControllerRotationYaw` true)))

(event `EnhancedInput|/Game/7_MISC/Input/IA_SpecialSkill`
  (params (ActionValue :type Boolean) (ElapsedSeconds :type "Float (double-precision)") (TriggeredSeconds :type "Float (double-precision)") (InputAction :type "InputAction Object Reference" :default "/Game/7_MISC/Input/IA_SpecialSkill.IA_SpecialSkill"))
  (:`Started`
    (`self.flameThrowerServer` :!label _label_4)))

(event `Key|Q`
  (params (Key :type "Key Structure"))
  (:`Pressed`
    (goto _label_4)))

(event `EnhancedInput|/Game/7_MISC/Input/IA_Basic_Roar`
  (params (ActionValue :type Boolean) (ElapsedSeconds :type "Float (double-precision)") (TriggeredSeconds :type "Float (double-precision)") (InputAction :type "InputAction Object Reference" :default "/Game/7_MISC/Input/IA_Basic_Roar.IA_Basic_Roar"))
  ;[1 1 1] Roar
  (:`Started`
    (`self.RoarAttack_Server` :!label _label_5)))

(event `Key|Three`
  (params (Key :type "Key Structure"))
  ;[1 1 1] Roar
  (:`Pressed`
    (goto _label_5)))

(event `flameThrowerServer`
  (`self.flameThrowerMulticast`))

(event `RoarAttack_Server`
  ;[1 1 1] Roar
  (`self.RoarAttack_Multicast`))

(event `flameThrowerMulticast`
  (if (`self.SCoolTime`)
    (`KismetSystemLibrary.PrintString` "coolTime!!!!" false true (struct :`R` 1.0 :`G` 0.960876 :`A` 1.0))
    (else
      (set `self.SCoolTime` true)
      (switch `int` (`self.SpecialSkill`)
        (:`Default`
          _)
        (:`0`
          _))
      (`|ExecutionSequence`
        (:`then_0`
          ;[1 0.5652 0.2997] 화염방사 스킬
          (`|PlayMontage` (`self.PlayerBody`) "/Game/7_MISC/Animation/Raptor/Skill/FireBreath/Raptor_BlueTRex_014_ck2_Anim_FireBreath_Montage3.Raptor_BlueTRex_014_ck2_Anim_FireBreath_Montage3" 1.0 0.0 "None"
            (:`then`
              (bind (_direction _firebreathaim) (`Timeline|Timeline_2` :!label _label_6)
                (:`Update`
                  (set `SpringArmComponent.TargetArmLength` (`KismetMathLibrary.Lerp` 600.0 500.0 _firebreathaim) (`self.PlayerCamArm`)))))
            (:`OnCompleted`
              (goto _label_6 :!via `Reverse`))))
        (:`then_1`
          ;[1 0.5652 0.2997] 화염방사 스킬
          (`ActorComponent.ToggleActive` (`self.SkillNiaEffect`))
          (set `self.bFlameOnOff` true)
          (`self.flameProjectileSpawner`)
          (`KismetSystemLibrary.Delay` (`self.SpecialCool`))
          (`ActorComponent.Deactivate` (`self.SkillNiaEffect`))
          (set `self.bFlameOnOff` false)
          (`KismetSystemLibrary.Delay` 0.2)
          (set `self.SCoolTime` false)
          (`KismetSystemLibrary.PrintString` "coolDown!!!!!!" false))))))

(event `RoarAttack_Multicast`
  ;[1 1 1] Roar
  (if (not (`self.bRoar`))
    (set `self.bRoar` true)
    (set `CharacterMovementComponent.MaxWalkSpeed` 0.0 (`self.CharacterMovement`))
    (set `self.bUseControllerRotationYaw` false)))

(event `RoarAttack_End`
  ;[1 1 1] Roar
  (if (`self.bRoar`)
    (set `self.bRoar` false)
    (set `CharacterMovementComponent.MaxWalkSpeed` 600.0 (`self.CharacterMovement`))
    (set `self.bUseControllerRotationYaw` true)))

(event `Key|Two`
  (params (Key :type "Key Structure"))
  ;[1 1 1] BiteAttack
  (:`Pressed`
    (`self.BiteAttack_Server` :!label _label_7)))

(event `EnhancedInput|/Game/7_MISC/Input/IA_Basic_Bite`
  (params (ActionValue :type Boolean) (ElapsedSeconds :type "Float (double-precision)") (TriggeredSeconds :type "Float (double-precision)") (InputAction :type "InputAction Object Reference" :default "/Game/7_MISC/Input/IA_Basic_Bite.IA_Basic_Bite"))
  ;[1 1 1] BiteAttack
  (:`Started`
    (goto _label_7)))

(event `BiteAttack_Server`
  ;[1 1 1] BiteAttack
  (`self.BiteAttack_Multicast`))

(event `BiteAttack_Multicast`
  ;[1 1 1] BiteAttack
  (if (not (`self.bBite`))
    (set `self.bBite` true)
    (`|PlayMontage` (`self.PlayerBody`) "/Game/7_MISC/Animation/Raptor/Skill/Bite/Raptor_Bite_Montage.Raptor_Bite_Montage"
      (:`OnCompleted`
        (if (`self.bBite`)
          (set `self.bBite` false))))))

(event `Key|E`
  (params (Key :type "Key Structure"))
  ;[1 0.8963 0.3185] Buff Skill
  (:`Pressed`
    (`self.BuffSkillServer`)))

(event `BuffSkillMulticast`
  (bind _tempstat (`self.tempStat`))
  ;[1 0.8963 0.3185] Buff Skill
  (set `self.coolTimeIndex` 3)
  (if (`self.BCoolTime`)
    (`KismetSystemLibrary.PrintString` "buff cool time !!!!!" false)
    (else
      (set `self.BCoolTime` true)
      (switch `int` (`self.currBuffskillNum`)
        (:`0`
          (bind _output_get (set `self.tempStat` (`self.powerStat`)))
          (set `self.powerStat` (+ _output_get 3.0)))
        (:`1`
          (bind _output_get_2 (set `self.tempStat` (`self.defenceStat`)))
          (set `self.defenceStat` (+ _output_get_2 3.0)))
        (:`2`
          (bind _output_get_3 (set `self.tempStat` (`self.speedStat`)))
          (set `self.speedStat` (+ _output_get_3 3.0))
          (set `CharacterMovementComponent.MaxWalkSpeed` (* 150.0 (`self.speedStat`)) (`self.CharacterMovement`))))
      (`self.buffSkillEffectMaker`)
      (`ActorComponent.SetActive` (`self.BuffEffect`) true false)
      (`KismetSystemLibrary.Delay` (`self.buffCool`))
      (switch `int` (`self.currBuffskillNum`)
        (:`0`
          (set `self.powerStat` _tempstat))
        (:`1`
          (set `self.defenceStat` _tempstat))
        (:`2`
          (set `self.speedStat` _tempstat)
          (set `CharacterMovementComponent.MaxWalkSpeed` (* 150.0 (`self.speedStat`)) (`self.CharacterMovement`))))
      (`ActorComponent.SetActive` (`self.BuffEffect`) false false)
      (`KismetSystemLibrary.Delay` 0.2)
      (set `self.BCoolTime` false))))

(event `BuffSkillServer`
  ;[1 0.8963 0.3185] Buff Skill
  (`self.BuffSkillMulticast`))

(fn `buffSkillEffectMaker`
  (switch `int` (`self.currBuffskillNum`)
    (:`Default`
      (bind _returnvalue (`NiagaraFunctionLibrary.SpawnSystemAttached` "/Game/5_FX/NS_PowerBuffEffect.NS_PowerBuffEffect" (`self.CapsuleComponent`) "None" (0.0 -0.0 -88.0) (struct :`Yaw` 90.0) "KeepRelativeOffset" false false :!label _label))
      (set `self.BuffEffect` _returnvalue))
    (:`0`
      (goto _label))
    (:`1`
      (bind _returnvalue_2 (`NiagaraFunctionLibrary.SpawnSystemAttached` "/Game/5_FX/NS_HealBuffEffect.NS_HealBuffEffect" (`self.CapsuleComponent`) "None" (0.0 -0.0 -88.0) (struct) "KeepRelativeOffset" false false))
      (set `self.BuffEffect` _returnvalue_2))
    (:`2`
      (bind _returnvalue_3 (`NiagaraFunctionLibrary.SpawnSystemAttached` "/Game/5_FX/NS_SpeedBuffEffect.NS_SpeedBuffEffect" (`self.CapsuleComponent`) "None" (0.0 -0.0 -88.0) (struct) "KeepRelativeOffset" false false))
      (set `self.BuffEffect` _returnvalue_3))))

(fn `HitMarkerMaker`)

(fn `playHitSound`
  (locals (sound2Play :type "SoundBase Object Reference"))
  (switch `int` (`KismetMathLibrary.RandomIntegerInRange` 0 2)
    (:`0`
      (set `local.sound2Play` "/Game/8_SOUND/DinoHitSound/Smash_Hit_Sound_Effects_HD__mp3cut_net_.Smash_Hit_Sound_Effects_HD__mp3cut_net_"))
    (:`1`
      (set `local.sound2Play` "/Game/8_SOUND/DinoHitSound/Smash_Hit_Sound_Effects_HD__mp3cut_net___1_.Smash_Hit_Sound_Effects_HD__mp3cut_net___1_"))
    (:`2`
      (set `local.sound2Play` "/Game/8_SOUND/DinoHitSound/Smash_Hit_Sound_Effects_HD__mp3cut_net___2_.Smash_Hit_Sound_Effects_HD__mp3cut_net___2_")))
  (`GameplayStatics.PlaySoundAtLocation` (`local.sound2Play`) (`self.K2_GetActorLocation`) (struct) 1.0 1.0 0.0 "/Game/8_SOUND/PlayerSoundAttenuation.PlayerSoundAttenuation" null null null))

(fn `SpecialSkillEffectMaker`
  (switch `int` (`self.SpecialSkill`)
    (:`0`
      (bind _returnvalue (`NiagaraFunctionLibrary.SpawnSystemAttached` "/Game/DragonFlameFX/FX/NS_DragonFlame_Fire1.NS_DragonFlame_Fire1" (`self.PlayerBody`) "Jaw" (0.0 0.0 0.0) (struct :`Pitch` -20.0) "KeepRelativeOffset" false false))
      (set `self.SkillNiaEffect` _returnvalue))
    (:`1`
      (bind _returnvalue_2 (`NiagaraFunctionLibrary.SpawnSystemAttached` "/Game/5_FX/VFX_Laser1.VFX_Laser1" (`self.PlayerBody`) "LaserBeam_Point" (0.0 0.0 0.0) (`KismetMathLibrary.Conv_VectorToRotator` (* (`SceneComponent.GetForwardVector` (`self.PlayerBody`)) (-1.0 0.0 0.0))) "KeepRelativeOffset" false false))
      (set `self.SkillNiaEffect` _returnvalue_2))
    (:`2`
      (`GameplayStatics.SpawnEmitterAtLocation` "/Game/5_FX/P_IceGroundAttack17.P_IceGroundAttack17" (0.0 0.0 0.0) (struct) (1.0 1.5 1.5) false "None" false))))

(fn `UserConstructionScript`
  (`SceneComponent.K2_AttachToComponent` (`self.PlayerTailCollision`) (`self.PlayerBody`) "Tail3" "KeepRelative" "KeepRelative" "KeepRelative" true)
  (`SceneComponent.K2_AttachToComponent` (`self.PlayerHeadCollision`) (`self.PlayerBody`) "Head" "KeepRelative" "KeepRelative" "KeepRelative" true))