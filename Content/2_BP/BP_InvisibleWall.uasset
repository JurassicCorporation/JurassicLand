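; BP_InvisibleWall is an actor that keeps itself positioned between the BP_BlueTRex actors in the level.
; It gathers those actors once, three seconds after BeginPlay.
; Each tick, when at least two were found and the first is valid, it moves to their average location and rotates toward the first one, using its pre-move position for the look-at.
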(event `self.ReceiveBeginPlay`
  (`KismetSystemLibrary.Delay` 3.0)
  (bind _outactors (`GameplayStatics.GetAllActorsOfClass` "/Game/2_BP/BP_BlueTRex.BP_BlueTRex_C"))
  (set `self.players` _outactors))

(event `self.ReceiveTick`
  (params (DeltaSeconds :type "Float (single-precision)"))
  (bind _output (`|GetArrayItem` (`self.players`)))
  (if (>= (`KismetArrayLibrary.Array_Length` (`self.players`)) 2)
    (bind _returnvalue (`GameplayStatics.GetActorArrayAverageLocation` (`self.players`)))
    (`/Engine/EditorBlueprintResources/StandardMacros.IsValid` _output
      (:`Is Valid`
        (`self.K2_SetActorLocationAndRotation` _returnvalue (`KismetMathLibrary.FindLookAtRotation` (`self.K2_GetActorLocation`) (`self.K2_GetActorLocation` _output)))))))

(fn `UserConstructionScript`)