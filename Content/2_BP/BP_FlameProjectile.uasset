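; BP_FlameProjectile is a short-lived flame projectile whose damage logic expects a BP_BlueTRex owner.
; It grows every tick and keeps its sphere collision off briefly after spawn before enabling it.
; Hitting anything but its owner applies fire damage from the owner's PowerStat, triggers the owner's hit marker, spawns a spark effect and destroys the projectile.
; An overlap-based damage path and an electric destruction effect are left disconnected.
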(event `self.ReceiveBeginPlay`
  (`self.SetLifeSpan` 1.0)
  (`PrimitiveComponent.SetCollisionEnabled` (`self.Sphere`) "NoCollision")
  (`KismetSystemLibrary.Delay` 0.2)
  (`PrimitiveComponent.SetCollisionEnabled` (`self.Sphere`) "QueryAndPhysics"))

(event `self.ReceiveTick`
  (params (DeltaSeconds :type "Float (single-precision)"))
  (`self.SetActorScale3D` (`self.scale`))
  (set `self.scale` (+ (`self.scale`) 0.05)))

(event `self.ReceiveActorBeginOverlap`
  (params (OtherActor :type "Actor Object Reference")))

(event `self.ReceiveHit`
  (params (MyComp :type "PrimitiveComponent Object Reference") (Other :type "Actor Object Reference") (OtherComp :type "PrimitiveComponent Object Reference") (bSelfMoved :type Boolean) (HitLocation :type "Vector Structure") (HitNormal :type "Vector Structure") (NormalImpulse :type "Vector Structure") (Hit :type "HitResult Structure (by ref)"))
  (bind (_bblockinghit _binitialoverlap _time _distance _location _impactpoint _normal) (`GameplayStatics.BreakHitResult` Hit))
  (bind _returnvalue (`self.GetOwner`))
  (if (!= Other _returnvalue)
    (bind _asbp_blue_trex (cast `/Game/2_BP/BP_BlueTRex` _returnvalue))
    (`GameplayStatics.ApplyDamage` Other (* (`/Game/2_BP/BP_BlueTRex.powerStat` _asbp_blue_trex) 1.0) null (`self.Instigator`) "/Game/2_BP/DamageType/DT_Fire.DT_Fire_C")
    (bind _asbp_blue_trex_2 (cast `/Game/2_BP/BP_BlueTRex` (`self.GetOwner`)))
    (`/Game/2_BP/BP_BlueTRex.HitMarkerMaker` _asbp_blue_trex_2)
    (`NiagaraFunctionLibrary.SpawnSystemAtLocation` "/Game/Realistic_Starter_VFX_Pack_Niagara/Niagara/Explosion/NS_HitSpark.NS_HitSpark" _impactpoint (`KismetMathLibrary.Conv_VectorToRotator` _normal))
    (`self.K2_DestroyActor`)))

(fn `UserConstructionScript`)