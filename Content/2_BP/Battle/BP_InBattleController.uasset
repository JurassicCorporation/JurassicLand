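; BP_InBattleController is the in-battle controller that sets up the local player's battle HUD.
; On BeginPlay it casts the player character to BP_BlueTRex, then for the local controller creates the battle and blood-effect widgets, passing the battle widget to the character.
; It also switches to game-only input with a hidden cursor.
; Tick polls the net game instance's IsEnd flag to remove the blood overlay and show the cursor.
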(event `self.ReceiveBeginPlay`
  (bind _returnvalue (`GameplayStatics.GetPlayerController` 0))
  (bind _asbp_blue_trex (cast `/Game/2_BP/BP_BlueTRex` (`GameplayStatics.GetPlayerCharacter` 0))
    (:`then`
      (if (`self.IsLocalController`)
        (bind _returnvalue_2 (`|CreateWidget` "/Game/2_BP/Widget/WBP_BattleWidget.WBP_BattleWidget_C"))
        (set `BlueTrex.battleUI` _returnvalue_2 _asbp_blue_trex)
        (bind _output_get (set `self.battlewidget` _returnvalue_2))
        (`UserWidget.AddToViewport` _output_get 0)
        (`WidgetBlueprintLibrary.SetInputMode_GameOnly` _returnvalue)
        (set `PlayerController.bShowMouseCursor` false _returnvalue)
        (`self.EnableInput` _returnvalue)
        (bind _returnvalue_3 (`|CreateWidget` "/Game/2_BP/Widget/inBattle/WB_BloodEffect.WB_BloodEffect_C"))
        (bind _output_get_2 (set `self.blood hit widget` _returnvalue_3))
        (`UserWidget.AddToViewport` _output_get_2 0)))
    (:`CastFailed`
      (`KismetSystemLibrary.PrintString` "Notbluetrex"))))

(event `self.ReceiveTick`
  (params (DeltaSeconds :type "Float (single-precision)"))
  (bind _blood_hit_widget (`self.blood hit widget`))
  (bind _asbp_lsh_net_game_instance (cast `/Game/LSH_WorkSpace/BP_LSH_NetGameInstance` (`GameplayStatics.GetGameInstance`)))
  (if (`LSH_NetGameInstance.isEnd` _asbp_lsh_net_game_instance)
    (`/Engine/EditorBlueprintResources/StandardMacros.IsValid` _blood_hit_widget
      (:`Is Valid`
        (`Widget.RemoveFromParent` _blood_hit_widget)
        (set `PlayerController.bShowMouseCursor` true (`GameplayStatics.GetPlayerController` 0))))))

(fn `UserConstructionScript`)